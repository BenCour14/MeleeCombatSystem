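; Frost boss enemy Blueprint that extends a parent mob enemy with a weapon and an on-screen boss health bar.
; The health widget binds to the stats component and shows while the boss has a target and is not dead.
; Left and right weapon collision hits apply stat-based point damage to receptive actors.
; The weapon mesh switches sockets when combat toggles and simulates physics on death.
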(event `self.ReceiveBeginPlay`
  (`parent.ReceiveBeginPlay`)
  (`/Game/CombatSystem/Blueprints/Components/BP_CollisionComponent.Set Collision Mesh` (`self.BP_RightWeaponCollisionComponent`) (`self.WeaponMesh`))
  (bind _returnvalue (`|CreateWidget` "/Game/CombatSystem/UI/WBP_BossHealth.WBP_BossHealth_C" (`GameplayStatics.GetPlayerController` 0)))
  (bind _output_get (set `self.BossHealthUI` _returnvalue))
  (`/Game/CombatSystem/UI/WBP_BossHealth.Initialize` _output_get (`self.BP_StatsComponent`))
  (`UserWidget.AddToViewport` (`self.BossHealthUI`) 0))

(event `SetBossHealthVisibility`
  (params (`bVisible?` :type Boolean))
  (bind _bosshealthui (`self.BossHealthUI`)
    (:`then`
      (`Widget.SetVisibility` _bosshealthui (select `bool` (and (not (`/Game/CombatSystem/Blueprints/Components/BP_StateManagerComponent.IsCurrentStateEqualToAny?` (`self.BP_StateManagerComponent`) (struct :`GameplayTags` (struct :`(TagName` "Character.State.Dead"))))) `bVisible?`) :`false` "Hidden" :`true` "Visible" :!type "ESlateVisibility Enum")))
    (:`else`)))

(event `/Game/CombatSystem/Blueprints/Interfaces/BPI_Targeting.OnTargeted`
  (params (`bIsTargeted?` :type Boolean))
  (`parent.OnTargeted` `bIsTargeted?`))

(event `HitEvent`
  (params (HitResult :type "HitResult Structure"))
  (bind (_bblockinghit _binitialoverlap _time _distance _location _impactpoint _normal _impactnormal _physmat _hitactor) (`GameplayStatics.BreakHitResult` HitResult))
  ;[0 0 0] Damage
  (bind _returnvalue (message `/Game/CombatSystem/Blueprints/Interfaces/BPI_Combat.CanReceiveDamage` _hitactor))
  (if _returnvalue
    (`GameplayStatics.ApplyPointDamage` _hitactor (`/Game/CombatSystem/Blueprints/Components/BP_StatsComponent.GetCurrentStatValue` (`self.BP_StatsComponent`) "NewEnumerator4") (`self.GetActorForwardVector`) HitResult (`self.GetController`) self "/Game/CombatSystem/Blueprints/DamageTypes/BP_AttackDamageType.BP_AttackDamageType_C")))

(event `self.BP_RightWeaponCollisionComponent.OnHit`
  (params (HitResult :type "HitResult Structure"))
  ;[0 0 0] Damage
  (`self.HitEvent` HitResult))

(event `self.BP_LeftWeaponCollisionComponent.OnHit`
  (params (HitResult :type "HitResult Structure"))
  ;[0 0 0] Damage
  (`self.HitEvent` HitResult))

(event `self.BP_CombatComponent.OnCombatToggled`
  (params (bIsCombatEnabled :type Boolean))
  ;[0 0 0] Toggle
  (`SceneComponent.K2_AttachToComponent` (`self.WeaponMesh`) (`self.Mesh`) (select `bool` bIsCombatEnabled :`false` (`self.Attach Socket Name`) :`true` (`self.Weapon Hand Socket Name`)) "SnapToTarget" "SnapToTarget" "SnapToTarget" true))

(event `Simulate Weapon Physics`
  (bind _weaponmesh (`self.WeaponMesh`))
  ;[0 0 0] Death
  (`PrimitiveComponent.SetCollisionProfileName` _weaponmesh "PhysicsActor" true)
  (`PrimitiveComponent.SetSimulatePhysics` _weaponmesh true)
  (`PrimitiveComponent.SetCollisionResponseToChannel` (`self.WeaponMesh`) "ECC_Pawn" "ECR_Ignore"))

(event `self.Perform Death`
  ;[0 0 0] Death
  (`parent.Perform Death`)
  (`self.Simulate Weapon Physics`)
  (`self.SetBossHealthVisibility` false))

(event `self.OnTargetSet`
  (params (NewTarget :type "Actor Object Reference"))
  (`parent.OnTargetSet` NewTarget)
  (`self.SetBossHealthVisibility` (`KismetSystemLibrary.IsValid` NewTarget)))

(fn `UserConstructionScript`
  (`parent.UserConstructionScript`))