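; BP_HeavyMobEnemy is a weapon-wielding enemy that extends a parent enemy class with a health bar, melee damage and weapon handling.
; Its health bar widget reads the stats component and is shown or hidden as targeting changes.
; Weapon collision hits apply stat-based point damage to actors that can receive it.
; Toggling combat snaps the weapon mesh between hand and attach sockets, and death switches it to simulated physics that ignores pawns.
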(event `self.ReceiveBeginPlay`
  (`parent.ReceiveBeginPlay`)
  (`/Game/CombatSystem/Blueprints/Components/BP_CollisionComponent.Set Collision Mesh` (`self.BP_RightWeaponCollisionComponent`) (`self.WeaponMesh`))
  (bind _returnvalue (`|CreateWidget` "/Game/CombatSystem/UI/WBP_HealthBar.WBP_HealthBar_C" (`GameplayStatics.GetPlayerController` 0) (`self.BP_StatsComponent`)))
  (`WidgetComponent.SetWidget` (`self.HealthBar`) _returnvalue))

(event `/Game/CombatSystem/Blueprints/Interfaces/BPI_Targeting.OnTargeted`
  (params (`bIsTargeted?` :type Boolean))
  (`parent.OnTargeted` `bIsTargeted?`)
  (`SceneComponent.SetVisibility` (`self.HealthBar`) `bIsTargeted?` false))

(event `self.BP_RightWeaponCollisionComponent.OnHit`
  (params (HitResult :type "HitResult Structure"))
  (bind (_bblockinghit _binitialoverlap _time _distance _location _impactpoint _normal _impactnormal _physmat _hitactor) (`GameplayStatics.BreakHitResult` HitResult))
  (bind _returnvalue (message `/Game/CombatSystem/Blueprints/Interfaces/BPI_Combat.CanReceiveDamage` _hitactor))
  (if _returnvalue
    (`GameplayStatics.ApplyPointDamage` _hitactor (`/Game/CombatSystem/Blueprints/Components/BP_StatsComponent.GetCurrentStatValue` (`self.BP_StatsComponent`) "NewEnumerator4") (`self.GetActorForwardVector`) HitResult (`self.GetController`) self "/Game/CombatSystem/Blueprints/DamageTypes/BP_AttackDamageType.BP_AttackDamageType_C")))

(event `self.BP_CombatComponent.OnCombatToggled`
  (params (bIsCombatEnabled :type Boolean))
  (`SceneComponent.K2_AttachToComponent` (`self.WeaponMesh`) (`self.Mesh`) (select `bool` bIsCombatEnabled :`false` (`self.Attach Socket Name`) :`true` (`self.Weapon Hand Socket Name`)) "SnapToTarget" "SnapToTarget" "SnapToTarget" true))

(event `Simulate Weapon Physics`
  (bind _weaponmesh (`self.WeaponMesh`))
  (`PrimitiveComponent.SetCollisionProfileName` _weaponmesh "PhysicsActor" true)
  (`PrimitiveComponent.SetSimulatePhysics` _weaponmesh true)
  (`PrimitiveComponent.SetCollisionResponseToChannel` (`self.WeaponMesh`) "ECC_Pawn" "ECR_Ignore"))

(event `self.Perform Death`
  (`parent.Perform Death`)
  (`self.Simulate Weapon Physics`))

(fn `UserConstructionScript`
  (`parent.UserConstructionScript`))