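; Armor item actor for skeletal pieces that follow the owning character's animation through master pose.
; AttachActor snaps its skeletal mesh to a socket on the owner Character's mesh and sets that mesh as the master pose component.
; Equipping adds ArmorValue to a stat on the owner's BP_StatsComponent, and unequipping subtracts it.
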(fn `AttachActor`
  (params (SocketName :type Name))
  (`/Engine/EditorBlueprintResources/StandardMacros.IsValid` (`SkinnedMeshComponent.SkeletalMesh` (`self.ItemSkeletalMesh`))
    (:`Is Valid`
      (`SceneComponent.K2_AttachToComponent` (`self.ItemSkeletalMesh`) (`Character.Mesh` (cast `Character` (`self.GetOwner`) :!pure true)) (`local.SocketName`) "SnapToTarget" "SnapToTarget" "SnapToTarget" true)
      (`SkinnedMeshComponent.SetLeaderPoseComponent` (`self.ItemSkeletalMesh`) (`Character.Mesh` (cast `Character` (`self.GetOwner`) :!pure true)) false)
      (return))
    (:`Is Not Valid`
      (return))))

(fn `On Equipped`
  (`parent.On Equipped`)
  (`/Game/CombatSystem/Blueprints/Components/BP_StatsComponent.ModifyCurrentStatValue` (`self.GetComponentByClass` (`self.GetOwner`) "/Game/CombatSystem/Blueprints/Components/BP_StatsComponent.BP_StatsComponent_C") "NewEnumerator3" (`self.ArmorValue`) false))

(fn `OnUnequipped`
  (`parent.OnUnequipped`)
  (`/Game/CombatSystem/Blueprints/Components/BP_StatsComponent.ModifyCurrentStatValue` (`self.GetComponentByClass` (`self.GetOwner`) "/Game/CombatSystem/Blueprints/Components/BP_StatsComponent.BP_StatsComponent_C") "NewEnumerator3" (* (`self.ArmorValue`) -1.0) false))

(fn `UserConstructionScript`
  (`parent.UserConstructionScript`))