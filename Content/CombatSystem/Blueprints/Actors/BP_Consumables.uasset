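; BP_Consumables is a consumable item actor in the combat system, handling the use of the item by its owner.
; Its UseItem event sends a PerformCustomAction message to the owning actor with the UseItem action tag, the general action state tag and the item's UseItemMontage.
; The graph applies no item effect itself, and its BeginPlay, overlap and Tick events are disabled stubs.
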(event `self.UseItem`
  (message `/Game/CombatSystem/Blueprints/Interfaces/BPI_Combat.PerformCustomAction` (`self.GetOwner`) (struct :`TagName` "Character.Action.UseItem") (struct :`TagName` "Character.State.General Action State") (`self.UseItemMontage`) 1.0 false))

(fn `UserConstructionScript`
  (`parent.UserConstructionScript`))