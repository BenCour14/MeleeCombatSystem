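; BP_HealthPotion is a usable health potion item actor in the combat system.
; On BeginPlay it sends its maximum use count to its owner through an interface message to update the potion amount.
; When the item action runs with uses remaining, it asks the owner to play the use-item montage as a tagged custom action.
; Healing and use decrement are not handled in this graph, which also prints debug true/false strings.
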(event `self.ReceiveBeginPlay`
  (`parent.ReceiveBeginPlay`)
  (message `/Game/CombatSystem/Blueprints/Interfaces/BPI_Combat.UpdateHealthPotionAmount` (`self.GetOwner`) (`self.Max Number Of Uses`)))

(event `/Game/CombatSystem/Blueprints/Actors/BP_BaseEquippable.PerformItemAction`
  (if (> (`self.CurrentNumberOfUses`) 0)
    (`KismetSystemLibrary.PrintString` "true")
    (message `/Game/CombatSystem/Blueprints/Interfaces/BPI_Combat.PerformCustomAction` (`self.GetOwner`) (struct :`TagName` "Character.Action.UseItem") (struct :`TagName` "Character.State.General Action State") (`self.UseItemMontage`) 1.0 false)
    (else
      (`KismetSystemLibrary.PrintString` "false"))))

(fn `UserConstructionScript`
  (`parent.UserConstructionScript`))