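; BP_LockedDoor is a door actor that is removed when the player interacts with it while holding a key.
; Overlap of its collision box by BP_CombatCharacter enables the door's input and opens a gate; leaving reverses both.
; On Interact, it reads HasKey from New_GameInstance, then either destroys itself through the gate or plays a locked-door sound at its location.
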(event `self.ReceiveBeginPlay`
  (bind _asnew_game_instance (cast `/Game/CombatSystem/Blueprints/New_GameInstance` (`GameplayStatics.GetGameInstance`)))
  (set `self.GameInstanceRef` _asnew_game_instance))

(event `InputAction|Interact`
  (params (Key :type "Key Structure"))
  (:`Pressed`
    (if (`/Game/CombatSystem/Blueprints/New_GameInstance.HasKey?` (`self.GameInstanceRef`))
      (`/Engine/EditorBlueprintResources/StandardMacros.Gate` true :!label _label
        (:`Exit`
          (`self.K2_DestroyActor`)))
      (else
        (`GameplayStatics.PlaySoundAtLocation` "/Game/ImportedAssets/FX/lockedDoor_Cue.lockedDoor_Cue" (`self.K2_GetActorLocation`) (struct) 1.0 1.0 0.0 null null null null)))))

(event `self.BoxCollision.OnComponentBeginOverlap`
  (params (OverlappedComponent :type "PrimitiveComponent Object Reference") (OtherActor :type "Actor Object Reference") (OtherComp :type "PrimitiveComponent Object Reference") (OtherBodyIndex :type Integer) (bFromSweep :type Boolean) (SweepResult :type "HitResult Structure (by ref)"))
  (cast `/Game/CombatSystem/Blueprints/BP_CombatCharacter` OtherActor)
  (`self.EnableInput` (`GameplayStatics.GetPlayerController` 0))
  (goto _label :!via `Open`))

(event `self.BoxCollision.OnComponentEndOverlap`
  (params (OverlappedComponent :type "PrimitiveComponent Object Reference") (OtherActor :type "Actor Object Reference") (OtherComp :type "PrimitiveComponent Object Reference") (OtherBodyIndex :type Integer))
  (cast `/Game/CombatSystem/Blueprints/BP_CombatCharacter` OtherActor)
  (`self.DisableInput` (`GameplayStatics.GetPlayerController` 0))
  (goto _label :!via `Close`))

(fn `UserConstructionScript`)