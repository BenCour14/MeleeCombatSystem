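; BP_Key is a key pickup that the player collects with the Interact input while standing in its trigger box.
; Overlap by BP_CombatCharacter enables input and opens a gate; leaving reverses both.
; Pickup sets HasKey on New_GameInstance, plays a sound and destroys the actor.
; On BeginPlay it destroys itself if HasKey is already set, otherwise a looping timer spins it in steps.
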(event `self.ReceiveBeginPlay`
  (bind _asnew_game_instance (cast `/Game/CombatSystem/Blueprints/New_GameInstance` (`GameplayStatics.GetGameInstance`)))
  (bind _output_get (set `self.GameInstanceRef` _asnew_game_instance))
  (if (`/Game/CombatSystem/Blueprints/New_GameInstance.HasKey?` _output_get)
    (`self.K2_DestroyActor`)
    (else
      (`KismetSystemLibrary.K2_SetTimer` null "Rotate Actor" 0.1 true))))

(event `InputAction|Interact`
  (params (Key :type "Key Structure"))
  (:`Pressed`
    (`/Engine/EditorBlueprintResources/StandardMacros.Gate` true :!label _label
      (:`Exit`
        (set `/Game/CombatSystem/Blueprints/New_GameInstance.HasKey?` true (`self.GameInstanceRef`))
        (`GameplayStatics.PlaySoundAtLocation` "/Game/ImportedAssets/FX/KeyPickUp_Cue.KeyPickUp_Cue" (`self.K2_GetActorLocation`) (struct) 1.0 1.0 0.0 null null null null)
        (`self.K2_DestroyActor`)))))

(event `self.BoxCollision.OnComponentBeginOverlap`
  (params (OverlappedComponent :type "PrimitiveComponent Object Reference") (OtherActor :type "Actor Object Reference") (OtherComp :type "PrimitiveComponent Object Reference") (OtherBodyIndex :type Integer) (bFromSweep :type Boolean) (SweepResult :type "HitResult Structure (by ref)"))
  (cast `/Game/CombatSystem/Blueprints/BP_CombatCharacter` OtherActor)
  (`self.EnableInput` (`GameplayStatics.GetPlayerController` 0))
  (goto _label :!via `Open`))

(event `self.BoxCollision.OnComponentEndOverlap`
  (params (OverlappedComponent :type "PrimitiveComponent Object Reference") (OtherActor :type "Actor Object Reference") (OtherComp :type "PrimitiveComponent Object Reference") (OtherBodyIndex :type Integer))
  (cast `/Game/CombatSystem/Blueprints/BP_CombatCharacter` OtherActor)
  (`self.DisableInput` (`GameplayStatics.GetPlayerController` 0))
  (goto _label :!via `Close`))

(event `Rotate Actor`
  (`self.K2_AddActorWorldRotation` (struct :`Yaw` 15.0)))

(fn `UserConstructionScript`)