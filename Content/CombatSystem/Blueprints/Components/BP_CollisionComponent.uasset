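; Actor component that detects hits for the combat system by sweeping between two sockets on an assigned mesh, likely a weapon.
; While collision is enabled, Tick runs a multi-sphere object trace between the start and end sockets, skipping ignored actors.
; Each newly hit actor is recorded and reported once through OnHit.
; Enabling collision clears the hit list, so each activation window can hit an actor again.
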(event `self.ReceiveTick`
  (params (DeltaSeconds :type "Float (single-precision)"))
  (if (`self.bIsCollisionEnabled?`)
    (`self.Collision Trace`)))

(event `Set Collision Mesh`
  (params (MeshComponent :type "PrimitiveComponent Object Reference"))
  ;[0 0 0] Set Collision Mesh Component
  (set `self.CollisionMeshComponent` MeshComponent))

(event `Enable Collision`
  ;[0 0 0] Enable Collision
  (`self.Clear Hit Actors`)
  (set `self.bIsCollisionEnabled?` true))

(event `Disable Collision`
  ;[0 0 0] Disable Collision
  (set `self.bIsCollisionEnabled?` false))

(event `Clear Hit Actors`
  ;[0 0 0] Clear Hit Actors
  (`KismetArrayLibrary.Array_Clear` (`self.AlreadyHitActors`)))

(event `Collision Trace`
  (bind _collisionmeshcomponent (`self.CollisionMeshComponent`))
  ;[0 0 0] Collision Trace
  (bind _outhits (`KismetSystemLibrary.SphereTraceMultiForObjects` (`SceneComponent.GetSocketLocation` _collisionmeshcomponent (`self.Start Socket Name`)) (`SceneComponent.GetSocketLocation` _collisionmeshcomponent (`self.End Socket Name`)) (`self.TraceRadius`) (`self.Collision Object Types`) false (`self.Actors to Ignore`) (`self.Draw Debug Type`)))
  (for _array_element _outhits
    (bind _output_get (set `self.LastHit` _array_element))
    (bind (_bblockinghit _binitialoverlap _time _distance _location _impactpoint _normal _impactnormal _physmat _hitactor) (`GameplayStatics.BreakHitResult` _output_get))
    (if (not (`KismetArrayLibrary.Array_Contains` (`self.AlreadyHitActors`) _hitactor))
      (bind _output_get_2 (set `self.Hit Actor` _hitactor))
      (`KismetArrayLibrary.Array_Add` (`self.AlreadyHitActors`) _output_get_2)
      (`self.OnHit` (`self.LastHit`)))))

(fn `Add Actor to Ignore`
  (params (InActor :type "Actor Object Reference (by ref)"))
  (`KismetArrayLibrary.Array_AddUnique` (`self.Actors to Ignore`) InActor))

(fn `GetActorsToIgnore`
  (returns (ReturnValue :type "Array of Actor Object Reference"))
  (return (`self.Actors to Ignore`)))

(fn `GetAlreadyHitActors`
  (returns (ReturnValue :type "Array of Actor Object Reference"))
  (return (`self.AlreadyHitActors`)))

(fn `GetCollisionMeshComponent`
  (returns (ReturnValue :type "PrimitiveComponent Object Reference"))
  (return (`self.CollisionMeshComponent`)))

(fn `GetLastHit`
  (returns (ReturnValue :type "HitResult Structure"))
  (return (`self.LastHit`)))

(fn `IsCollisionEnabled`
  (returns (ReturnValue :type Boolean))
  (return (`self.bIsCollisionEnabled?`)))

(fn `Remove Actor to Ignore`
  (params (`Actor To Remove` :type "Actor Object Reference (by ref)"))
  (`KismetArrayLibrary.Array_RemoveItem` (`self.Actors to Ignore`) `Actor To Remove`))